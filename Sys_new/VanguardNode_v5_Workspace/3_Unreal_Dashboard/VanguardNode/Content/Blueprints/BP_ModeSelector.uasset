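; BP_ModeSelector is an actor that, on BeginPlay, fetches scan data over REST and uses it to build the level's spatial grid.
; It creates a Cpp_Rest_Bridge, binds its OnEventsFetched callback and calls FetchEvents.
; The handler prints and parses the JSON, then passes valid scan data to GenerateGridFromScan on the first BP_SpatialGrid found, with colored debug prints for success or failure.
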(event Custom|HandleScanResponse
  (params (JsonResponse :type String))
  (Development|PrintString JsonResponse true true "(R=0.000000,G=0.660000,B=1.000000,A=1.000000)" 15.0)
  (bind (_outscandata _returnvalue) (Class|CppRestBridge|ParseScanJson JsonResponse))
  (if _returnvalue
    (bind _outactors (Actor|GetAllActorsOfClass "/Game/Blueprints/BP_SpatialGrid.BP_SpatialGrid_C"))
    (Development|PrintString "Hello" true true "(R=0.842601,G=1.000000,B=0.000000,A=1.000000)")
    (Default|GenerateGridfromScan (Utilities|Array|Get(acopy) _outactors) _outscandata)
    (else
      (Development|PrintString "Hello" true true "(R=1.000000,G=0.064729,B=0.000000,A=1.000000)"))))

(event EventBeginPlay
  (bind _returnvalue (Game|ConstructObjectfromClass "/Script/VanguardNode.Cpp_Rest_Bridge" self))
  (bind _output_get (Variables|Default|SetRestBridgeInstance _returnvalue))
  (EventDispatchers|BindEventtoOnEventsFetched _returnvalue (delegate Custom|HandleScanResponse))
  (Class|CppRestBridge|FetchEvents _returnvalue))

(event Collision|EventActorBeginOverlap
  (params (OtherActor :type Actor%20Object%20Reference)))

(event EventTick
  (params (DeltaSeconds :type Float%20%28single-precision%29)))

(fn ConstructionScript)