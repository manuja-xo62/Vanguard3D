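; BP_NetworkManager is an actor that polls a local scan API over HTTP and caches the latest result.
; From BeginPlay, a looping Delay fires a VaRest GET request several times a second, without waiting for the previous response.
; The completion callback reads target file, issue count and predicted risk score from the JSON into LatestScanData, then prints debug messages including the score.
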(event Custom|FetchScanData
  (bind _returnvalue (Class|VaRestSubsystem|ConstructVaRestRequestExt (|VaRestSubsystem) "GET" "json"))
  (Class|VaRestRequestJSON|SetURL _returnvalue "http://127.0.0.1:5000/api/scan")
  (EventDispatchers|BindEventtoOnRequestComplete _returnvalue (delegate Custom|OnScanResponseRecieved))
  (Class|VaRestRequestJSON|ExecuteProcessRequest _returnvalue))

(event Custom|OnScanResponseRecieved
  (params (Request :type Va%20Rest%20Request%20JSON%20Object%20Reference))
  (bind _returnvalue (Class|VaRestRequestJSON|GetResponseObject Request))
  (Development|PrintString "Hello")
  (bind _output_get (Variables|Default|SetLatestScanData (Utilities|Struct|MakeS_ScanResponse "" (Class|VaRestJsonObject|GetStringField _returnvalue "target_file") (Class|VaRestJsonObject|GetIntegerField _returnvalue "total_issues") (Class|VaRestJsonObject|GetNumberField _returnvalue "predicted_risk_score") 0)))
  (Development|PrintString (Utilities|String|Append "Scan Complete! Risk Score: " (Utilities|String|ToString(Float) (.predicted_risk_score _output_get)))))

(event EventBeginPlay
  (CallFunction|FetchScanData :!label _label)
  (Utilities|FlowControl|Delay 0.2)
  (goto _label))

(event Collision|EventActorBeginOverlap
  (params (OtherActor :type Actor%20Object%20Reference)))

(event EventTick
  (params (DeltaSeconds :type Float%20%28single-precision%29)))

(fn ConstructionScript)