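; Spatial grid Blueprint that visualises scanned files as instanced static meshes.
; GenerateGridFromScan clears previous results, then places one instance per file in rows and columns by array index, so skipped .vanguard_backup files leave gaps.
; It writes each file's RFile, divided by 100, to instance custom data, using the array index as the data slot.
; FileFinding records entries keyed by array index, and scan ID and paths print for debugging.
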(event Custom|GenerateGridFromScan
  (params (ScanData :type Scan%20Response%20Structure))
  (bind (_status _scan_id _data) (Utilities|Struct|BreakScanResponse ScanData))
  (bind _columnsperrow (Variables|Default|GetColumnsPerRow))
  (bind _grid_spacing (Variables|Default|GetGrid%20Spacing))
  (bind _ism_filecontainers (Variables|Default|GetISM_FileContainers))
  (Components|InstancedStaticMesh|ClearInstances (Variables|Default|GetISM_FileContainers))
  (Utilities|Map|Clear (Variables|Default|GetFileFinding))
  (Development|PrintString _scan_id)
  (for (_array_element _array_index) (.files (Utilities|Struct|BreakScanDataWrapper _data))
    (if (not (Utilities|String|Contains (.file_path (Utilities|Struct|BreakFileFinding _array_element)) ".vanguard_backup" true))
      (Development|PrintString (.file_path (Utilities|Struct|BreakFileFinding _array_element)) true true "(R=0.000000,G=0.660000,B=1.000000,A=1.000000)" 1e+01)
      (bind _returnvalue (Components|InstancedStaticMesh|AddInstance _ism_filecontainers (Math|Transform|MakeTransform (Math|Vector|MakeVector (* (Math|Integer|%(Integer) _array_index _columnsperrow) _grid_spacing) (* (/ _array_index _columnsperrow) _grid_spacing) 0.0))))
      (Components|InstancedStaticMesh|SetCustomDataValue _ism_filecontainers _returnvalue _array_index (/ (.R_file (Utilities|Struct|BreakFileFinding _array_element)) 1e+02) false)
      (Utilities|Map|Add :TargetMap (Variables|Default|GetFileFinding) :Key _array_index))))

(event EventBeginPlay)

(event Collision|EventActorBeginOverlap
  (params (OtherActor :type Actor%20Object%20Reference)))

(event EventTick
  (params (DeltaSeconds :type Float%20%28single-precision%29)))

(fn ConstructionScript)