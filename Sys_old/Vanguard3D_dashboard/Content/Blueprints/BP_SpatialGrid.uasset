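; BP_SpatialGrid is an actor that visualises scan telemetry as a grid of instanced static meshes.
; On BeginPlay it binds to the scan-completed event of the first BP_VanguardBackend_Manager found.
; Each scan rebuilds a three-column grid, one instance per vulnerability with a minimum of one.
; Global risk score sets the shared material: amber for the middle band, crimson for both high and low bands.
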(event Custom|ByuldGridFromTelemetry
  (params (GlobalRiskScore :type Float%20%28single-precision%29) (VulnerbilityCount :type Integer) (TargetFile :type String))
  (bind _instancedstaticmesh (Variables|Default|GetInstancedStaticMesh))
  (Components|InstancedStaticMesh|ClearInstances _instancedstaticmesh)
  (for _index (range 0 (- (Math|Integer|Max(Integer) VulnerbilityCount 1) 1))
    (Components|InstancedStaticMesh|AddInstance _instancedstaticmesh (Math|Transform|MakeTransform (Math|Vector|MakeVector (Math|Conversions|ToFloat(Integer) (* (Math|Integer|%(Integer) _index 3) 250)) (Math|Conversions|ToFloat(Integer) (* (/ _index 3) 250)) 0.0))))
  (if (>= GlobalRiskScore 75.0)
    (Rendering|Material|SetMaterial _instancedstaticmesh 0 "/Game/Blueprints/Materials/RiskMaterials/MI_Container_Crimson.MI_Container_Crimson")
    (elif (>= GlobalRiskScore 3e+01)
      (Rendering|Material|SetMaterial _instancedstaticmesh 0 "/Game/Blueprints/Materials/RiskMaterials/MI_Container_Amber.MI_Container_Amber")
      (else
        (Rendering|Material|SetMaterial _instancedstaticmesh 0 "/Game/Blueprints/Materials/RiskMaterials/MI_Container_Crimson.MI_Container_Crimson")))))

(event EventBeginPlay
  (bind _outactors (Actor|GetAllActorsOfClass "/Game/Blueprints/BP_VanguardBackend_Manager.BP_VanguardBackend_Manager_C"))
  (EventDispatchers|BindEventtoOnScanCompleted (Utilities|Array|Get(acopy) _outactors) (delegate Custom|ByuldGridFromTelemetry)))

(event Collision|EventActorBeginOverlap
  (params (OtherActor :type Actor%20Object%20Reference)))

(event EventTick
  (params (DeltaSeconds :type Float%20%28single-precision%29)))

(fn ConstructionScript)