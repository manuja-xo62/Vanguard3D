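; BP_VanguardBackend_Manager is an actor that bridges the game to a local HTTP security-scanning backend through VaRest.
; On BeginPlay it prints the health-check status, then after a short delay posts a scan request.
; The scan response's risk score, vulnerability count and file path are broadcast through the OnScanCompleted dispatcher.
; A Patch event posts to the patch endpoint, but its response handler is empty.
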(event Custom|FetchScanData
  (bind _returnvalue (Class|VaRestSubsystem|ConstructVaRestRequestExt (|VaRestSubsystem) "GET" "json"))
  (Class|VaRestRequestJSON|SetURL _returnvalue "http://127.0.0.1:8000/health")
  (EventDispatchers|BindEventtoOnRequestComplete _returnvalue (delegate Custom|OnScanResponseRecieved))
  (Class|VaRestRequestJSON|ExecuteProcessRequest _returnvalue))

(event Custom|OnScanResponseRecieved
  (params (Request :type Va%20Rest%20Request%20JSON%20Object%20Reference))
  (Development|PrintString (Class|VaRestJsonObject|GetStringField (Class|VaRestRequestJSON|GetResponseObject Request) "status")))

(event Custom|ExecuteScan
  (bind _returnvalue (Class|VaRestSubsystem|ConstructVaRestRequestExt (|VaRestSubsystem) "POST" "json"))
  (Class|VaRestRequestJSON|SetURL _returnvalue "http://127.0.0.1:8000/api/scan")
  (EventDispatchers|BindEventtoOnRequestComplete _returnvalue (delegate Custom|OnScanResponseReceived))
  (Class|VaRestRequestJSON|ExecuteProcessRequest _returnvalue))

(event Custom|OnScanResponseReceived
  (params (Request :type Va%20Rest%20Request%20JSON%20Object%20Reference))
  (bind _returnvalue (Class|VaRestRequestJSON|GetResponseObject Request))
  (Default|CallOnScanCompleted (Class|VaRestJsonObject|GetNumberField _returnvalue "global_risk_score") (Math|Float|Truncate (Class|VaRestJsonObject|GetNumberField _returnvalue "vulnerabilities_found")) (Class|VaRestJsonObject|GetStringField _returnvalue "file_path")))

(event Custom|Patch
  (bind _returnvalue (Class|VaRestSubsystem|ConstructVaRestRequestExt (|VaRestSubsystem) "POST" "json"))
  (Class|VaRestRequestJSON|SetURL _returnvalue "http://127.0.0.1:8000/api/patch")
  (EventDispatchers|BindEventtoOnRequestComplete _returnvalue (delegate Custom|OnPatchResponseReceived))
  (Class|VaRestRequestJSON|ExecuteProcessRequest _returnvalue))

(event Custom|OnPatchResponseReceived
  (params (Request :type Va%20Rest%20Request%20JSON%20Object%20Reference)))

(event EventBeginPlay
  (CallFunction|FetchScanData)
  (Utilities|FlowControl|Delay 3.0)
  (CallFunction|ExecuteScan))

(event Collision|EventActorBeginOverlap
  (params (OtherActor :type Actor%20Object%20Reference)))

(event EventTick
  (params (DeltaSeconds :type Float%20%28single-precision%29)))

(fn ConstructionScript)